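; BP_Ball is the ball in a Pong-style game, launched along Y at BeginPlay by setting its mesh's physics velocity.
; Overlap events drive bouncing through casts: either paddle reverses Y and sets X to the paddle's velocity plus a random offset.
; Horizontal boundaries reverse X.
; Either goal recenters the ball at the world origin and relaunches it along Y, in opposite directions for left and right goals.
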(event `self.ReceiveBeginPlay`
  (`PrimitiveComponent.SetPhysicsLinearVelocity` (`self.StaticMesh`) (0.0 2500.0 0.0) false "None"))

(event `self.ReceiveActorBeginOverlap`
  (params (OtherActor :type "Actor Object Reference"))
  (bind _asbp_paddle_pawn_right (cast `/Game/Blueprints/BP_Paddle_Pawn_Right` OtherActor)
    (:`then`
      (bind _returnvalue (`PrimitiveComponent.GetPhysicsLinearVelocity` (`/Game/Blueprints/BP_Paddle_Pawn_Right.Paddle_Mesh` _asbp_paddle_pawn_right) "None"))
      (bind _returnvalue_2 (`PrimitiveComponent.GetPhysicsLinearVelocity` (`self.StaticMesh`) "None"))
      (`PrimitiveComponent.SetPhysicsLinearVelocity` (`self.StaticMesh`) (`KismetMathLibrary.MakeVector` (+ (.x _returnvalue) (`KismetMathLibrary.RandomFloatInRange` -1000.0 1000.0)) (* (.y _returnvalue_2) -1.0) (.z _returnvalue_2)) false "None"))
    (:`CastFailed`
      (bind _asbp_enemy_paddle (cast `/Game/Blueprints/BP_EnemyPaddle` OtherActor)
        (:`then`
          (bind _returnvalue_3 (`PrimitiveComponent.GetPhysicsLinearVelocity` (`/Game/Blueprints/BP_EnemyPaddle.StaticMesh` _asbp_enemy_paddle) "None"))
          (bind _returnvalue_4 (`PrimitiveComponent.GetPhysicsLinearVelocity` (`self.StaticMesh`) "None"))
          (`PrimitiveComponent.SetPhysicsLinearVelocity` (`self.StaticMesh`) (`KismetMathLibrary.MakeVector` (+ (.x _returnvalue_3) (`KismetMathLibrary.RandomFloatInRange` -1000.0 1000.0)) (* (.y _returnvalue_4) -1.0) (.z _returnvalue_4)) false "None"))
        (:`CastFailed`
          (cast `/Game/Blueprints/BP_Horizontal_Boundary` OtherActor
            (:`then`
              (bind _returnvalue_5 (`PrimitiveComponent.GetPhysicsLinearVelocity` (`self.StaticMesh`) "None"))
              (`PrimitiveComponent.SetPhysicsLinearVelocity` (`self.StaticMesh`) (`KismetMathLibrary.MakeVector` (* (.x _returnvalue_5) -1.0) (.y _returnvalue_5) (.z _returnvalue_5)) false "None"))
            (:`CastFailed`
              (cast `/Game/Blueprints/BP_L_Goal` OtherActor
                (:`then`
                  (`self.K2_SetActorLocation` (0.0 0.0 0.0))
                  (`PrimitiveComponent.SetPhysicsLinearVelocity` (`self.StaticMesh`) (0.0 2000.0 0.0) false "None"))
                (:`CastFailed`
                  (cast `/Game/Blueprints/BP_R_Goal` OtherActor)
                  (`self.K2_SetActorLocation` (0.0 0.0 0.0))
                  (`PrimitiveComponent.SetPhysicsLinearVelocity` (`self.StaticMesh`) (0.0 -2000.0 0.0) false "None"))))))))))

(fn `UserConstructionScript`)