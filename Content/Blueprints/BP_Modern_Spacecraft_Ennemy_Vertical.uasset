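; BP_Modern_Spacecraft_Ennemy_Vertical is an AI-driven enemy spacecraft that follows BP_ModernBall actors along the world X axis.
; Every Tick it finds all balls and, for each, applies a physics impulse to SpacecraftMesh from the clamped X offset times AILeftSpacecraftSpeed.
; Impulses from multiple balls accumulate, and none are scaled by delta time, so movement depends on frame rate.
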(event `self.ReceiveTick`
  (params (DeltaSeconds :type "Float (single-precision)"))
  (bind _outactors (`GameplayStatics.GetAllActorsOfClass` "/Game/Blueprints/BP_ModernBall.BP_ModernBall_C"))
  (for _array_element _outactors
    (`PrimitiveComponent.AddImpulse` (`self.Spacecraft_mesh`) (* (`KismetMathLibrary.MakeVector` (`KismetMathLibrary.FClamp` (- (.x (`self.K2_GetActorLocation` _array_element)) (.x (`self.K2_GetActorLocation`))) -8000.0 8000.0)) (`self.AI_LeftSpacecraftSpeed`)) "None" false)))

(fn `UserConstructionScript`)