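; Physics ball for a four-sided Pong variant, launched on BeginPlay.
; Overlaps with spacecraft paddles rebound it using randomized boosts and paddle velocity; pillar hits apply the pillar's negated X/Y velocity.
; Tick checks the overlap event's OtherActor against bounds, recentering that actor, relaunching the ball and decrementing that side's score, or reloads a ClassicPong level after GameOver.
; Score text and loss checks, the only GameOver setters, are unwired.
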(event `self.ReceiveBeginPlay`
  (`PrimitiveComponent.SetPhysicsLinearVelocity` (`self.StaticMesh`) (-2500.0 -1500.0 0.0) false "None"))

(event `self.ReceiveActorBeginOverlap`
  (params (OtherActor :type "Actor Object Reference"))
  (bind _returnvalue (`KismetMathLibrary.RandomFloatInRange` 1.1 1.5))
  (bind _returnvalue_2 (`KismetMathLibrary.RandomFloatInRange` 1.1 1.5))
  (bind _returnvalue_3 (`KismetMathLibrary.RandomFloatInRange` 1.1 1.5))
  (bind _asbp_modern_spacecraft_bottom (cast `/Game/Blueprints/Modern/BP_Modern_Spacecraft_Bottom` OtherActor)
    (:`then`
      (bind _returnvalue_4 (`PrimitiveComponent.GetPhysicsLinearVelocity` (`/Game/Blueprints/Modern/BP_Modern_Spacecraft_Bottom.Spacecraft_mesh` _asbp_modern_spacecraft_bottom) "None"))
      (bind _returnvalue_5 (`PrimitiveComponent.GetPhysicsLinearVelocity` (`self.StaticMesh`) "None"))
      (`PrimitiveComponent.SetPhysicsLinearVelocity` (`self.StaticMesh`) (`KismetMathLibrary.MakeVector` (* (.x _returnvalue_5) _returnvalue -1.0) (* (.y _returnvalue_4) _returnvalue) (.z _returnvalue_5)) false "None")
      (`GameplayStatics.PlaySoundAtLocation` "/Game/Audio/S_ballCollision.S_ballCollision"))
    (:`CastFailed`
      (bind _asbp_modern_spacecraft_ennemy_vertical (cast `/Game/Blueprints/Modern/BP_Modern_Spacecraft_Ennemy_Vertical` OtherActor)
        (:`then`
          (bind _returnvalue_6 (`PrimitiveComponent.GetPhysicsLinearVelocity` (`/Game/Blueprints/Modern/BP_Modern_Spacecraft_Ennemy_Vertical.Spacecraft_mesh` _asbp_modern_spacecraft_ennemy_vertical) "None"))
          (bind _returnvalue_7 (`PrimitiveComponent.GetPhysicsLinearVelocity` (`self.StaticMesh`) "None"))
          (`PrimitiveComponent.SetPhysicsLinearVelocity` (`self.StaticMesh`) (`KismetMathLibrary.MakeVector` (* (.x _returnvalue_6) _returnvalue_3) (* (.y _returnvalue_7) _returnvalue_3 -1.0) (.z _returnvalue_7)) false "None")
          (`GameplayStatics.PlaySoundAtLocation` "/Game/Audio/S_ballCollision.S_ballCollision"))
        (:`CastFailed`
          (bind _asbp_modern_spacecraft_ennemy_horizontal (cast `/Game/Blueprints/Modern/BP_Modern_Spacecraft_Ennemy_Horizontal` OtherActor)
            (:`then`
              (bind _returnvalue_8 (`PrimitiveComponent.GetPhysicsLinearVelocity` (`/Game/Blueprints/Modern/BP_Modern_Spacecraft_Ennemy_Horizontal.Spacecraft_mesh` _asbp_modern_spacecraft_ennemy_horizontal) "None"))
              (bind _returnvalue_9 (`PrimitiveComponent.GetPhysicsLinearVelocity` (`self.StaticMesh`) "None"))
              (`PrimitiveComponent.SetPhysicsLinearVelocity` (`self.StaticMesh`) (`KismetMathLibrary.MakeVector` (* (.x _returnvalue_9) _returnvalue_2 -1.0) (* (.y _returnvalue_8) _returnvalue_2) (.z _returnvalue_9)) false "None")
              (`GameplayStatics.PlaySoundAtLocation` "/Game/Audio/S_ballCollision.S_ballCollision"))
            (:`CastFailed`
              (bind _asbp_pillar (cast `/Game/Blueprints/Modern/BP_Pillar` OtherActor))
              (bind _returnvalue_10 (`PrimitiveComponent.GetPhysicsLinearVelocity` (`/Game/Blueprints/Modern/BP_Pillar.StaticMesh` _asbp_pillar) "None"))
              (`PrimitiveComponent.SetPhysicsLinearVelocity` (`self.StaticMesh`) (`KismetMathLibrary.MakeVector` (* (.x _returnvalue_10) -1.0) (* (.y _returnvalue_10) -1.0) (.z _returnvalue_10)) false "None")
              (`GameplayStatics.PlaySoundAtLocation` "/Game/Audio/S_ballCollision.S_ballCollision"))))))))

(event `self.ReceiveTick`
  (params (DeltaSeconds :type "Float (single-precision)"))
  (if (`self.bGame_Over`)
    (`PrimitiveComponent.SetPhysicsLinearVelocity` (`self.StaticMesh`) (0.0 0.0 0.0) false "None")
    (`KismetSystemLibrary.Delay` 3.0)
    (bind _outactors (`GameplayStatics.GetAllActorsOfClass` "/Game/Blueprints/Classic/BP_Paddle_Left.BP_Paddle_Left_C"))
    (if (> (`KismetArrayLibrary.Array_Length` _outactors) 0)
      (`GameplayStatics.OpenLevel` "ClassicPong_P2_main")
      (else
        (`GameplayStatics.OpenLevel` "ClassicPong_P1_main")))
    (else
      (bind _returnvalue (`self.K2_GetActorLocation` (stale `self.ReceiveActorBeginOverlap` OtherActor)))
      (bind _x (.x _returnvalue))
      (bind _y (.y _returnvalue))
      (if (> _y 4000.0)
        (bind _returnvalue_2 (`KismetStringLibrary.Conv_VectorToString` _returnvalue))
        (`KismetSystemLibrary.PrintString` _returnvalue_2)
        (`self.K2_SetActorLocation` (stale `self.ReceiveActorBeginOverlap` OtherActor) (0.0 0.0 0.0) false false)
        (`PrimitiveComponent.SetPhysicsLinearVelocity` (`self.StaticMesh`) (1000.0 2000.0 0.0) false "None")
        (`GameplayStatics.PlaySoundAtLocation` "/Game/Audio/S_ballGoal.S_ballGoal")
        (set `self.rPlayer_Score` (- (`self.rPlayer_Score`) 1))
        (elif (< _y -4000.0)
          (`KismetSystemLibrary.PrintString` _returnvalue_2)
          (`self.K2_SetActorLocation` (stale `self.ReceiveActorBeginOverlap` OtherActor) (0.0 0.0 0.0) false false)
          (`PrimitiveComponent.SetPhysicsLinearVelocity` (`self.StaticMesh`) (1000.0 -2000.0 0.0) false "None")
          (`GameplayStatics.PlaySoundAtLocation` "/Game/Audio/S_ballGoal.S_ballGoal")
          (set `self.lPlayer_Score` (- (`self.lPlayer_Score`) 1))
          (elif (> _x 4000.0)
            (`KismetSystemLibrary.PrintString` _returnvalue_2)
            (`self.K2_SetActorLocation` (stale `self.ReceiveActorBeginOverlap` OtherActor) (0.0 0.0 0.0) false false)
            (`PrimitiveComponent.SetPhysicsLinearVelocity` (`self.StaticMesh`) (1000.0 2000.0 0.0) false "None")
            (`GameplayStatics.PlaySoundAtLocation` "/Game/Audio/S_ballGoal.S_ballGoal")
            (set `self.tPlayer_Score` (- (`self.tPlayer_Score`) 1))
            (elif (< _x -4000.0)
              (`KismetSystemLibrary.PrintString` _returnvalue_2)
              (`self.K2_SetActorLocation` (stale `self.ReceiveActorBeginOverlap` OtherActor) (0.0 0.0 0.0) false false)
              (`PrimitiveComponent.SetPhysicsLinearVelocity` (`self.StaticMesh`) (1000.0 -2000.0 0.0) false "None")
              (`GameplayStatics.PlaySoundAtLocation` "/Game/Audio/S_ballGoal.S_ballGoal")
              (set `self.bPlayer_Score` (- (`self.bPlayer_Score`) 1)))))))))

(fn `UserConstructionScript`)