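; BP_Modern_Spacecraft_Ennemy_Vertical is an AI-driven enemy spacecraft that tracks BP_ModernBall actors along world X.
; Each Tick it finds every ball and pushes SpacecraftMesh with an X-only impulse from the clamped ball offset, scaled by AIVerticalSpacecraftSpeed.
; If the craft strays beyond fixed X bounds, it resets to X zero, keeping Y and Z, instead of applying that impulse.
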(event `self.ReceiveTick`
  (params (DeltaSeconds :type "Float (single-precision)"))
  (bind _outactors (`GameplayStatics.GetAllActorsOfClass` "/Game/Blueprints/Modern/BP_ModernBall.BP_ModernBall_C"))
  (for _array_element _outactors
    (if (> (.x (`self.K2_GetActorLocation`)) 5000.0)
      (`self.K2_SetActorLocation` (`KismetMathLibrary.MakeVector` 0.0 (.y (`self.K2_GetActorLocation`)) (.z (`self.K2_GetActorLocation`))))
      (elif (< (.x (`self.K2_GetActorLocation`)) -5000.0)
        (`self.K2_SetActorLocation` (`KismetMathLibrary.MakeVector` 0.0 (.y (`self.K2_GetActorLocation`)) (.z (`self.K2_GetActorLocation`))))
        (else
          (`PrimitiveComponent.AddImpulse` (`self.Spacecraft_mesh`) (* (`KismetMathLibrary.MakeVector` (`KismetMathLibrary.FClamp` (- (.x (`self.K2_GetActorLocation` _array_element)) (.x (`self.K2_GetActorLocation`))) -8000.0 8000.0)) (`self.AI_VerticalSpacecraftSpeed`)) "None" false))))))

(fn `UserConstructionScript`)