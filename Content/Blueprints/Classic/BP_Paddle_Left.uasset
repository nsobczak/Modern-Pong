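; Left paddle actor for the Classic mode, moved along the X axis by the P2_MoveUp input axis.
; Each tick it applies a large physics force to its static mesh, scaled by the axis value.
; When the paddle passes either X limit, it is teleported just inside the bound and receives no force that frame.
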(event `self.ReceiveTick`
  (params (DeltaSeconds :type "Float (single-precision)"))
  (if (> (.x (`self.K2_GetActorLocation`)) 3250.0)
    (`self.K2_SetActorLocation` (`KismetMathLibrary.MakeVector` 3249.0 (.y (`self.K2_GetActorLocation`)) (.z (`self.K2_GetActorLocation`))))
    (elif (< (.x (`self.K2_GetActorLocation`)) -3250.0)
      (`self.K2_SetActorLocation` (`KismetMathLibrary.MakeVector` -3249.0 (.y (`self.K2_GetActorLocation`)) (.z (`self.K2_GetActorLocation`))))
      (else
        (`PrimitiveComponent.AddForce` (`self.StaticMesh`) (`KismetMathLibrary.MakeVector` (* (`self.GetInputAxisValue`) 300000000.0)) "None" false)))))

(fn `UserConstructionScript`)