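; Pong ball for classic mode that bounces off paddles and boundaries, keeps both players' scores and ends the match.
; Overlap casts pick the response: paddles reverse Y and set X from paddle velocity plus random spread, while boundaries reverse X.
; Goals recenter and relaunch the ball and update tagged TextRender scores, setting GameOver at five points.
; Tick then freezes the ball and, after a delay, opens the one- or two-player level depending on whether BP_Paddle_Left exists.
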(event `self.ReceiveBeginPlay`
  (`PrimitiveComponent.SetPhysicsLinearVelocity` (`self.StaticMesh`) (60.0 2500.0 0.0) false "None"))

(event `self.ReceiveActorBeginOverlap`
  (params (OtherActor :type "Actor Object Reference"))
  (bind _asbp_paddle_pawn_right (cast `/Game/Blueprints/Classic/BP_Paddle_Pawn_Right` OtherActor)
    (:`then`
      (bind _returnvalue (`PrimitiveComponent.GetPhysicsLinearVelocity` (`/Game/Blueprints/Classic/BP_Paddle_Pawn_Right.Paddle_Mesh` _asbp_paddle_pawn_right) "None"))
      (bind _returnvalue_2 (`PrimitiveComponent.GetPhysicsLinearVelocity` (`self.StaticMesh`) "None"))
      (`PrimitiveComponent.SetPhysicsLinearVelocity` (`self.StaticMesh`) (`KismetMathLibrary.MakeVector` (+ (.x _returnvalue) (`KismetMathLibrary.RandomFloatInRange` -1000.0 1000.0)) (* (.y _returnvalue_2) -1.0) (.z _returnvalue_2)) false "None")
      (`GameplayStatics.PlaySoundAtLocation` "/Game/Audio/S_ballCollision.S_ballCollision"))
    (:`CastFailed`
      (bind _asbp_paddle_left (cast `/Game/Blueprints/Classic/BP_Paddle_Left` OtherActor)
        (:`then`
          (bind _returnvalue_3 (`PrimitiveComponent.GetPhysicsLinearVelocity` (`/Game/Blueprints/Classic/BP_Paddle_Left.StaticMesh` _asbp_paddle_left) "None"))
          (bind _returnvalue_4 (`PrimitiveComponent.GetPhysicsLinearVelocity` (`self.StaticMesh`) "None"))
          (`PrimitiveComponent.SetPhysicsLinearVelocity` (`self.StaticMesh`) (`KismetMathLibrary.MakeVector` (+ (.x _returnvalue_3) (`KismetMathLibrary.RandomFloatInRange` -1000.0 1000.0)) (* (.y _returnvalue_4) -1.0) (.z _returnvalue_4)) false "None")
          (`GameplayStatics.PlaySoundAtLocation` "/Game/Audio/S_ballCollision.S_ballCollision"))
        (:`CastFailed`
          (bind _asbp_enemy_paddle (cast `/Game/Blueprints/Classic/BP_EnemyPaddle` OtherActor)
            (:`then`
              (bind _returnvalue_5 (`PrimitiveComponent.GetPhysicsLinearVelocity` (`/Game/Blueprints/Classic/BP_EnemyPaddle.StaticMesh` _asbp_enemy_paddle) "None"))
              (bind _returnvalue_6 (`PrimitiveComponent.GetPhysicsLinearVelocity` (`self.StaticMesh`) "None"))
              (`PrimitiveComponent.SetPhysicsLinearVelocity` (`self.StaticMesh`) (`KismetMathLibrary.MakeVector` (+ (.x _returnvalue_5) (`KismetMathLibrary.RandomFloatInRange` -1000.0 1000.0)) (* (.y _returnvalue_6) -1.0) (.z _returnvalue_6)) false "None")
              (`GameplayStatics.PlaySoundAtLocation` "/Game/Audio/S_ballCollision.S_ballCollision"))
            (:`CastFailed`
              (cast `/Game/Blueprints/Classic/BP_Horizontal_Boundary` OtherActor
                (:`then`
                  (bind _returnvalue_7 (`PrimitiveComponent.GetPhysicsLinearVelocity` (`self.StaticMesh`) "None"))
                  (`PrimitiveComponent.SetPhysicsLinearVelocity` (`self.StaticMesh`) (`KismetMathLibrary.MakeVector` (* (.x _returnvalue_7) -1.0) (.y _returnvalue_7) (.z _returnvalue_7)) false "None")
                  (`GameplayStatics.PlaySoundAtLocation` "/Game/Audio/S_ballCollision.S_ballCollision"))
                (:`CastFailed`
                  (cast `/Game/Blueprints/Classic/BP_L_Goal` OtherActor
                    (:`then`
                      (`self.K2_SetActorLocation` (0.0 0.0 0.0))
                      (`PrimitiveComponent.SetPhysicsLinearVelocity` (`self.StaticMesh`) (0.0 2000.0 0.0) false "None")
                      (`GameplayStatics.PlaySoundAtLocation` "/Game/Audio/S_ballGoal.S_ballGoal")
                      (set `self.rPlayer_Score` (+ (`self.rPlayer_Score`) 1))
                      (bind _outactors (`GameplayStatics.GetAllActorsOfClass` "/Script/Engine.TextRenderActor"))
                      (for _array_element _outactors
                        (bind _textrender (`TextRenderActor.TextRender` _array_element))
                        (if (`ActorComponent.ComponentHasTag` _textrender "R_Player_Score_Tag")
                          (`TextRenderComponent.K2_SetText` _textrender (`KismetTextLibrary.Conv_IntToText` (`self.rPlayer_Score`)))
                          (if (> (`self.rPlayer_Score`) 4)
                            (`KismetSystemLibrary.PrintString` "Right side wins")
                            (set `self.bGameOver` true)))))
                    (:`CastFailed`
                      (cast `/Game/Blueprints/Classic/BP_R_Goal` OtherActor)
                      (`self.K2_SetActorLocation` (0.0 0.0 0.0))
                      (`PrimitiveComponent.SetPhysicsLinearVelocity` (`self.StaticMesh`) (0.0 -2000.0 0.0) false "None")
                      (`GameplayStatics.PlaySoundAtLocation` "/Game/Audio/S_ballGoal.S_ballGoal")
                      (set `self.lPlayer_Score` (+ (`self.lPlayer_Score`) 1))
                      (bind _outactors_2 (`GameplayStatics.GetAllActorsOfClass` "/Script/Engine.TextRenderActor"))
                      (for _array_element_2 _outactors_2
                        (bind _textrender_2 (`TextRenderActor.TextRender` _array_element_2))
                        (if (`ActorComponent.ComponentHasTag` _textrender_2 "L_Player_Score_Tag")
                          (`TextRenderComponent.K2_SetText` _textrender_2 (`KismetTextLibrary.Conv_IntToText` (`self.lPlayer_Score`)))
                          (if (> (`self.lPlayer_Score`) 4)
                            (`KismetSystemLibrary.PrintString` "Left side wins")
                            (set `self.bGameOver` true)))))))))))))))

(event `self.ReceiveTick`
  (params (DeltaSeconds :type "Float (single-precision)"))
  (if (`self.bGameOver`)
    (`PrimitiveComponent.SetPhysicsLinearVelocity` (`self.StaticMesh`) (0.0 0.0 0.0) false "None")
    (`KismetSystemLibrary.Delay` 3.0)
    (bind _outactors (`GameplayStatics.GetAllActorsOfClass` "/Game/Blueprints/Classic/BP_Paddle_Left.BP_Paddle_Left_C"))
    (if (> (`KismetArrayLibrary.Array_Length` _outactors) 0)
      (`GameplayStatics.OpenLevel` "ClassicPong_P2_main")
      (else
        (`GameplayStatics.OpenLevel` "ClassicPong_P1_main")))))

(fn `UserConstructionScript`)